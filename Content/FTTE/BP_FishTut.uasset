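; Interactable fishing tutorial trigger that shows the WBP_FishTut widget when the player presses E nearby.
; A box overlap stores the player and toggles an indicator, while BeginPlay creates the widget once and binds the character's E-press and the widget's close events.
; Opening disables character movement and switches to UI-only input with a cursor.
; Closing removes the widget and restores walking and game-only input.
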(event `CloseTut`
  (bind _returnvalue (`GameplayStatics.GetPlayerController` 0))
  (`Widget.RemoveFromParent` (`self.TutWidget`))
  (set `self.bTutOpen` false)
  (`CharacterMovementComponent.SetMovementMode` (`Character.CharacterMovement` (`self.playerRef`)) "MOVE_Walking" 0)
  (set `PlayerController.bShowMouseCursor` false _returnvalue)
  (`WidgetBlueprintLibrary.SetInputMode_GameOnly` _returnvalue))

(event `self.ReceiveBeginPlay`
  (`SceneComponent.SetVisibility` (`self.InteractIndicator`) false false)
  (bind _returnvalue (`|CreateWidget` "/Game/FTTE/Widgets/WBP_FishTut.WBP_FishTut_C"))
  (set `self.TutWidget` _returnvalue)
  (bind _asbp_third_person_character (cast `/Game/FTTE/BP_ThirdPersonCharacter` (`GameplayStatics.GetPlayerPawn` 0)))
  (add `/Game/FTTE/BP_ThirdPersonCharacter.EPressed` _asbp_third_person_character (delegate `EPressed`))
  (add `/Game/FTTE/Widgets/WBP_FishTut.CloseTut` (`self.TutWidget`) (delegate `CloseTut`)))

(event `EPressed`
  (bind _returnvalue (`GameplayStatics.GetPlayerController` 0))
  (bind _tutwidget (`self.TutWidget`))
  (if (`self.bPlayerInRange`)
    (if (not (`self.bTutOpen`))
      (set `self.bTutOpen` true)
      (`UserWidget.AddToViewport` _tutwidget 0)
      (`CharacterMovementComponent.SetMovementMode` (`Character.CharacterMovement` (`self.playerRef`)) "MOVE_None" 0)
      (set `PlayerController.bShowMouseCursor` true _returnvalue)
      (`WidgetBlueprintLibrary.SetInputMode_UIOnlyEx` _returnvalue _tutwidget))))

(event `self.Box.OnComponentBeginOverlap`
  (params (OverlappedComponent :type "PrimitiveComponent Object Reference") (OtherActor :type "Actor Object Reference") (OtherComp :type "PrimitiveComponent Object Reference") (OtherBodyIndex :type Integer) (bFromSweep :type Boolean) (SweepResult :type "HitResult Structure (by ref)"))
  (bind _asbp_third_person_character (cast `/Game/FTTE/BP_ThirdPersonCharacter` OtherActor))
  (set `self.bPlayerInRange` true)
  (`SceneComponent.SetVisibility` (`self.InteractIndicator`) true false)
  (set `self.PlayerRef` _asbp_third_person_character))

(event `self.Box.OnComponentEndOverlap`
  (params (OverlappedComponent :type "PrimitiveComponent Object Reference") (OtherActor :type "Actor Object Reference") (OtherComp :type "PrimitiveComponent Object Reference") (OtherBodyIndex :type Integer))
  (set `self.bPlayerInRange` false)
  (`SceneComponent.SetVisibility` (`self.InteractIndicator`) false false))

(fn `UserConstructionScript`)