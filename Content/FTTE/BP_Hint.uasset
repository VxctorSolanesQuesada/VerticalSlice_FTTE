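; BP_Hint is a pickup actor that unlocks a fish hint for the player.
; A Sphere overlap with BP_ThirdPersonCharacter stores the character and flags it in range; any end overlap clears the flag without checking which actor left.
; On BeginPlay it binds to the player character's E-pressed event.
; Pressing E in range passes FishHintID to SetFishHasHintByID on the character, then destroys the hint.
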(event `self.ReceiveBeginPlay`
  (bind _asbp_third_person_character (cast `/Game/ThirdPerson/Blueprints/BP_ThirdPersonCharacter` (`GameplayStatics.GetPlayerPawn` 0)))
  (add `/Game/ThirdPerson/Blueprints/BP_ThirdPersonCharacter.EPressed` _asbp_third_person_character (delegate `EPressed`)))

(event `EPressed`
  (bind _playerref (`self.PlayerRef`))
  (if (`self.bPlayerInRange`)
    (`/Engine/EditorBlueprintResources/StandardMacros.IsValid` _playerref
      (:`Is Valid`
        (`/Game/ThirdPerson/Blueprints/BP_ThirdPersonCharacter.SetFishHasHintByID` _playerref (`self.FishHintID`))
        (`self.K2_DestroyActor`)))))

(event `self.Sphere.OnComponentBeginOverlap`
  (params (OverlappedComponent :type "PrimitiveComponent Object Reference") (OtherActor :type "Actor Object Reference") (OtherComp :type "PrimitiveComponent Object Reference") (OtherBodyIndex :type Integer) (bFromSweep :type Boolean) (SweepResult :type "HitResult Structure (by ref)"))
  (bind _asbp_third_person_character (cast `/Game/ThirdPerson/Blueprints/BP_ThirdPersonCharacter` OtherActor))
  (set `self.bPlayerInRange` true)
  (set `self.PlayerRef` _asbp_third_person_character))

(event `self.Sphere.OnComponentEndOverlap`
  (params (OverlappedComponent :type "PrimitiveComponent Object Reference") (OtherActor :type "Actor Object Reference") (OtherComp :type "PrimitiveComponent Object Reference") (OtherBodyIndex :type Integer))
  (set `self.bPlayerInRange` false))

(fn `UserConstructionScript`)