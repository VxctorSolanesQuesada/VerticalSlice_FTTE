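; BP_Inventory stores the player's caught fish and their running total value, and owns the inventory widget.
; BeginPlay creates WBP_Inventory and loads it from this Blueprint, and the I key toggles it on screen.
; AddFish adds the price to the total, stacks fish by FishID or appends new ones, then reloads the widget and prints the total.
; ShowEncyclopedia is an empty stub.
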(event `self.ReceiveBeginPlay`
  (bind _asbp_third_person_character (cast `/Game/ThirdPerson/Blueprints/BP_ThirdPersonCharacter` (`GameplayStatics.GetPlayerPawn` 0)))
  (set `self.PlayerRef` _asbp_third_person_character)
  (bind _returnvalue (`|CreateWidget` "/Game/FTTE/Widgets/WBP_Inventory.WBP_Inventory_C"))
  (set `self.InventoryWidget` _returnvalue)
  (`/Game/FTTE/Widgets/WBP_Inventory.LoadInventory` (`self.InventoryWidget`) self))

(event `Key|I`
  (params (Key :type "Key Structure"))
  (bind _inventorywidget (`self.InventoryWidget`))
  (:`Pressed`
    (if (`Widget.IsVisible` (`self.InventoryWidget`))
      (`Widget.RemoveFromParent` _inventorywidget)
      (else
        (`UserWidget.AddToViewport` _inventorywidget 0)))))

(fn `AddFish`
  (params (NewFish :type "/Game/FTTE/ST_FishData Structure"))
  (locals (PezActual :type Integer :default 0))
  (bind (_name _rarity _price _zone _count _fishid) (break `/Game/FTTE/ST_FishData` NewFish))
  (set `self.InventoryValor` (+ (`self.InventoryValor`) _price))
  (set `self.bIsCaught` false)
  (for (_array_element _array_index) (`self.FishInventory`)
    (if (== (`.FishID_21_7588424F45B0D9C5021CE7BD8BAE89C6` (break `/Game/FTTE/ST_FishData` _array_element)) _fishid)
      (set `self.bIsCaught` true)
      (bind _result (`/Engine/EditorBlueprintResources/StandardMacros.IncrementInt` (`.Count_19_94EFD7844C21E1945BE6B7AB6C36A018` (break `/Game/FTTE/ST_FishData` _array_element)))
        (:`  `
          (bind _structout (setmembers `/Game/FTTE/ST_FishData` :`StructRef` _array_element :`Count` _result))
          (`KismetArrayLibrary.Array_Set` (`self.FishInventory`) _array_index _structout)
          (`/Game/FTTE/Widgets/WBP_Inventory.LoadInventory` (`self.InventoryWidget`) self :!label _label)
          (`KismetSystemLibrary.PrintString` (`KismetStringLibrary.Conv_IntToString` (`self.InventoryValor`)))))))
  (if (not (`self.bIsCaught`))
    (`KismetArrayLibrary.Array_Add` (`self.FishInventory`) NewFish)
    (goto _label)))

(fn `ShowEncyclopedia`)