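; Shop actor that sells lava-resistant fishing bait to the player through a WBP_Buy dialogue widget.
; A box overlap tracks the player, whose E-press dispatcher opens the widget, halts movement and shows the cursor until closed.
; Widget dispatchers drive closing and buying, which checks Money against BaitPrice and enables CanFishInLava without deducting coins here.
; A successful purchase closes the shop and blocks reopening; insufficient funds changes the dialogue text.
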(event `CloseShop`
  (bind _returnvalue (`GameplayStatics.GetPlayerController` 0))
  (`Widget.RemoveFromParent` (`self.BuyWidget`))
  (set `self.bShopOpen` false)
  (`CharacterMovementComponent.SetMovementMode` (`Character.CharacterMovement` (`self.playerRef`)) "MOVE_Walking" 0)
  (set `PlayerController.bShowMouseCursor` false _returnvalue)
  (`WidgetBlueprintLibrary.SetInputMode_GameOnly` _returnvalue))

(event `self.ReceiveBeginPlay`
  (bind _returnvalue (`|CreateWidget` "/Game/FTTE/Widgets/WBP_Buy.WBP_Buy_C"))
  (set `self.BuyWidget` _returnvalue)
  (bind _asbp_third_person_character (cast `/Game/ThirdPerson/Blueprints/BP_ThirdPersonCharacter` (`GameplayStatics.GetPlayerPawn` 0)))
  (add `/Game/ThirdPerson/Blueprints/BP_ThirdPersonCharacter.EPressed` _asbp_third_person_character (delegate `EPressed`))
  (add `/Game/FTTE/Widgets/WBP_Buy.CloseBuy` (`self.BuyWidget`) (delegate `CloseShop`))
  (add `/Game/FTTE/Widgets/WBP_Buy.BuyLavaBait` (`self.BuyWidget`) (delegate `BuyLava`)))

(event `BuyLava`
  (bind _playerref (`self.PlayerRef`))
  (if (>= (`/Game/ThirdPerson/Blueprints/BP_ThirdPersonCharacter.Money` _playerref) (`self.BaitPrice`))
    (set `/Game/ThirdPerson/Blueprints/BP_ThirdPersonCharacter.bCanFishInLava` true _playerref)
    (`KismetSystemLibrary.PrintString` "Fish Lava ON!")
    (`/Game/FTTE/Widgets/WBP_Buy.CloseBuy` (`self.BuyWidget`))
    (set `self.bAllBought` true)
    (else
      (`TextBlock.SetText` (`/Game/FTTE/Widgets/WBP_Buy.TalkBox` (`self.BuyWidget`)) "Oops! \nYou’ll need 500 coins to get this bait. \n \nCome back when you have enough money, and I’ll be right here waiting for you!"))))

(event `EPressed`
  (bind _returnvalue (`GameplayStatics.GetPlayerController` 0))
  (if (`self.bPlayerInRange`)
    (if (`self.bAllBought`)
      _
      (elif (not (`self.bShopOpen`))
        (set `self.bShopOpen` true)
        (`UserWidget.AddToViewport` (`self.BuyWidget`) 0)
        (`CharacterMovementComponent.SetMovementMode` (`Character.CharacterMovement` (`self.playerRef`)) "MOVE_None" 0)
        (set `PlayerController.bShowMouseCursor` true _returnvalue)
        (`WidgetBlueprintLibrary.SetInputMode_GameAndUIEx` _returnvalue null "DoNotLock" false)
        (`TextBlock.SetText` (`/Game/FTTE/Widgets/WBP_Buy.TalkBox` (`self.BuyWidget`)) "Hello there, adventurer! \nPlanning to fish in lava? Then you’ll need something special! This lava-resistant fishing bait can handle the heat and help you catch the rarest fiery fish. \n \nIt’s strong, shiny, and totally safe for extreme fishing… and it only costs 500 coins! Wanna give it a try?")))))

(event `self.Box.OnComponentBeginOverlap`
  (params (OverlappedComponent :type "PrimitiveComponent Object Reference") (OtherActor :type "Actor Object Reference") (OtherComp :type "PrimitiveComponent Object Reference") (OtherBodyIndex :type Integer) (bFromSweep :type Boolean) (SweepResult :type "HitResult Structure (by ref)"))
  (bind _asbp_third_person_character (cast `/Game/ThirdPerson/Blueprints/BP_ThirdPersonCharacter` OtherActor))
  (set `self.bPlayerInRange` true)
  (set `self.PlayerRef` _asbp_third_person_character))

(event `self.Box.OnComponentEndOverlap`
  (params (OverlappedComponent :type "PrimitiveComponent Object Reference") (OtherActor :type "Actor Object Reference") (OtherComp :type "PrimitiveComponent Object Reference") (OtherBodyIndex :type Integer))
  (set `self.bPlayerInRange` false))

(fn `UserConstructionScript`)