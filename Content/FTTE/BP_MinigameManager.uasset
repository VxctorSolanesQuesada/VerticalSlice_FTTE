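; BP_MinigameManager runs a fishing minigame built around a meter that drains over time and must be filled to win.
; StartMinigame creates the WBP_FishingHud widget and starts a looping timer, used instead of Tick, that drains the meter and refreshes the HUD.
; RegisterHit and RegisterMiss raise or lower the meter with sound feedback.
; Reaching the maximum fires OnWin and hitting the minimum fires OnFail, both stopping the timer and removing the HUD.
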(fn `RegisterHit`
  (bind _fishingwidgedref (`self.FishingWidgedRef`))
  (if (`self.bActive`)
    (bind _output_get (set `self.Meter` (+ (`self.Meter`) (`self.HitReward`))))
    (`GameplayStatics.PlaySound2D` "/Game/SFX/SFX_Good.SFX_Good" 1.0 1.0 0.0 null null)
    (if (>= _output_get (`self.MeterMax`))
      (set `self.bActive` false)
      (`KismetSystemLibrary.K2_ClearAndInvalidateTimerHandle` (`self.UpdateTimerHandle`))
      (`self.OnWin`)
      (`/Engine/EditorBlueprintResources/StandardMacros.IsValid` _fishingwidgedref
        (:`Is Valid`
          (`Widget.RemoveFromParent` _fishingwidgedref))))
    (else
      (return))))

(fn `RegisterMiss`
  (if (`self.bActive`)
    (set `self.Meter` (- (`self.Meter`) (`self.LoseReward`)))
    (`GameplayStatics.PlaySound2D` "/Game/SFX/SFX_Wrong.SFX_Wrong" 1.0 1.0 0.0 null null)
    (else
      (return))))

(fn `StartMinigame`
  (set `self.bActive` true)
  (set `self.Meter` (`self.StartMeter`))
  (`KismetSystemLibrary.K2_ClearAndInvalidateTimerHandle` (`self.UpdateTimerHandle`))
  (bind _returnvalue (`KismetSystemLibrary.K2_SetTimer` null "UpdateMeter" (`self.UpdateRate`) true))
  (set `self.UpdateTimerHandle` _returnvalue)
  (bind _returnvalue_2 (`|CreateWidget` "/Game/FTTE/Widgets/WBP_FishingHud.WBP_FishingHud_C" (`GameplayStatics.GetPlayerController` 0)))
  (bind _output_get (set `self.FishingWidgedRef` _returnvalue_2))
  (`UserWidget.AddToViewport` _output_get 0)
  (`/Game/FTTE/Widgets/WBP_FishingHud.UpdateMeter` _output_get (`self.Meter`) (`self.MeterMax`)))

(fn `UpdateMeter`
  (bind _fishingwidgedref (`self.FishingWidgedRef`))
  (if (`self.bActive`)
    (set `self.Meter` (`KismetMathLibrary.FClamp` (- (`self.Meter`) (* (`self.DrainPerSecond`) (`self.UpdateRate`))) (`self.MeterMin`) (`self.MeterMax`)))
    (`/Engine/EditorBlueprintResources/StandardMacros.IsValid` (`self.FishingWidgedRef`)
      (:`Is Valid`
        (`/Game/FTTE/Widgets/WBP_FishingHud.UpdateMeter` (`self.FishingWidgedRef`) (`self.Meter`) (`self.MeterMax`))
        (if (<= (`self.Meter`) (`self.MeterMin`))
          (set `self.bActive` false)
          (`KismetSystemLibrary.K2_ClearAndInvalidateTimerHandle` (`self.UpdateTimerHandle`))
          (`self.OnFail`)
          (`/Engine/EditorBlueprintResources/StandardMacros.IsValid` _fishingwidgedref
            (:`Is Valid`
              (`Widget.RemoveFromParent` _fishingwidgedref)))
          (else
            (return)))))
    (else
      (return))))